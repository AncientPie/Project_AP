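; Notebook interactable that shows a note on screen when the player presses the interact key near it.
; Overlapping the Box with player_BP enables input and shows the Interacción_IF prompt widget; leaving disables input and removes it.
; Pressing Interacción swaps the prompt for a Notas_IF widget with Taku's text, which is removed after a short delay.
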(event `self.Box.OnComponentBeginOverlap`
  (params (OverlappedComponent :type "PrimitiveComponent Object Reference") (OtherActor :type "Actor Object Reference") (OtherComp :type "PrimitiveComponent Object Reference") (OtherBodyIndex :type Integer) (bFromSweep :type Boolean) (SweepResult :type "HitResult Structure (by ref)"))
  ;[1 1 1] Cuando el jugador entra en la caja de colisión del cuaderno, aparece el texto
  (cast `/Game/Blueprints/player_BP` OtherActor)
  (`self.EnableInput` (`GameplayStatics.GetPlayerController` 0))
  (bind _returnvalue (`|CreateWidget` "/Game/Interfaces/Interacción_IF.Interacción_IF_C"))
  (`UserWidget.AddToViewport` _returnvalue 0))

(event `InputAction|Interacción`
  (params (Key :type "Key Structure"))
  ;[1 1 1] Aparece texto de Taku
  (:`Pressed`
    (`Widget.RemoveFromParent` (stale `self.Box.OnComponentBeginOverlap` _returnvalue))
    (bind _returnvalue (`|CreateWidget` "/Game/Interfaces/notas_IF.notas_IF_C"))
    (`UserWidget.AddToViewport` _returnvalue 0)
    (`KismetSystemLibrary.Delay` 3.0)
    (`Widget.RemoveFromParent` _returnvalue)))

(event `self.Box.OnComponentEndOverlap`
  (params (OverlappedComponent :type "PrimitiveComponent Object Reference") (OtherActor :type "Actor Object Reference") (OtherComp :type "PrimitiveComponent Object Reference") (OtherBodyIndex :type Integer))
  ;[1 1 1] Cuando el jugador sale de la caja de colisión, desaparece el texto
  (cast `/Game/Blueprints/player_BP` OtherActor)
  (`self.DisableInput` null)
  (`Widget.RemoveFromParent` (stale `self.Box.OnComponentBeginOverlap` _returnvalue)))

(fn `UserConstructionScript`)