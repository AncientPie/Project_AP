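; Player Blueprint for a sprite-based character that moves along world X and Y from two input axes.
; MoveHorizontal and MoveVertical each add movement input, then read velocity to pick the Sprite's flipbook.
; Horizontal logic sets idle when still and right or left walk for sideways or diagonal motion.
; Vertical logic handles pure Y motion, choosing the Run or Climb flipbook by direction.
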(event `InputAxis|MoveHorizontal`
  (params (AxisValue :type "Float (single-precision)"))
  (bind (_returnvalue_x _returnvalue_y) (`KismetMathLibrary.BreakVector` (`self.GetVelocity`)))
  (bind _sprite (`self.Sprite`))
  (bind _returnvalue (== _returnvalue_y 0.0))
  (bind _returnvalue_2 (!= _returnvalue_x 0.0))
  ;[1 1 1] Movimiento (Anim)
  (`self.AddMovementInput` (1.0 0.0 0.0) AxisValue)
  (if (and (== _returnvalue_x 0.0) _returnvalue)
    (`PaperFlipbookComponent.SetFlipbook` _sprite "/Game/Flipbooks/Player_Flipbooks/idle_FB.idle_FB")
    (elif (and _returnvalue_2 _returnvalue)
      (if (> _returnvalue_x 0.0)
        (`PaperFlipbookComponent.SetFlipbook` _sprite "/Game/Flipbooks/Player_Flipbooks/walk_FB.walk_FB" :!label _label)
        (else
          (`PaperFlipbookComponent.SetFlipbook` _sprite "/Game/Flipbooks/Player_Flipbooks/walk_left_FB.walk_left_FB" :!label _label_2)))
      (elif (and _returnvalue_2 (!= _returnvalue_y 0.0))
        (if (> _returnvalue_x 0.0)
          (goto _label)
          (else
            (goto _label_2)))))))

(event `InputAxis|MoveVertical`
  (params (AxisValue :type "Float (single-precision)"))
  (bind (_returnvalue_x _returnvalue_y) (`KismetMathLibrary.BreakVector` (`self.GetVelocity`)))
  (bind _sprite (`self.Sprite`))
  ;[1 1 1] Movimiento (Anim)
  (`self.AddMovementInput` (0.0 -1.0 0.0) AxisValue)
  (if (and (== _returnvalue_x 0.0) (!= _returnvalue_y 0.0))
    (if (> _returnvalue_y 0.0)
      (`PaperFlipbookComponent.SetFlipbook` _sprite "/Game/Flipbooks/Player_Flipbooks/run_FB.run_FB")
      (else
        (`PaperFlipbookComponent.SetFlipbook` _sprite "/Game/Flipbooks/Player_Flipbooks/climb_FB.climb_FB")))))

(fn `UserConstructionScript`)