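; Door actor that lets the player travel to the bathroom level (Baño_lvl) by interacting with it.
; Overlapping its Box with player_BP enables input on the actor and shows an Interacción_IF prompt widget.
; The Interacción input action removes the prompt and opens the level by name.
; Leaving the Box disables input and removes the widget.
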(event `self.Box.OnComponentBeginOverlap`
  (params (OverlappedComponent :type "PrimitiveComponent Object Reference") (OtherActor :type "Actor Object Reference") (OtherComp :type "PrimitiveComponent Object Reference") (OtherBodyIndex :type Integer) (bFromSweep :type Boolean) (SweepResult :type "HitResult Structure (by ref)"))
  ;[1 1 1] Pulsa 'E' para interactuar y la interacción itself
  (cast `/Game/Blueprints/player_BP` OtherActor)
  (`self.EnableInput` (`GameplayStatics.GetPlayerController` 0))
  (bind _returnvalue (`|CreateWidget` "/Game/Interfaces/Interacción_IF.Interacción_IF_C"))
  (`UserWidget.AddToViewport` _returnvalue 0))

(event `InputAction|Interacción`
  (params (Key :type "Key Structure"))
  ;[1 1 1] Pulsa 'E' para interactuar y la interacción itself
  (:`Pressed`
    (`Widget.RemoveFromParent` (stale `self.Box.OnComponentBeginOverlap` _returnvalue))
    (`GameplayStatics.OpenLevel` "Baño_lvl")))

(event `self.Box.OnComponentEndOverlap`
  (params (OverlappedComponent :type "PrimitiveComponent Object Reference") (OtherActor :type "Actor Object Reference") (OtherComp :type "PrimitiveComponent Object Reference") (OtherBodyIndex :type Integer))
  ;[1 1 1] Pulsa 'E' para interactuar y la interacción itself
  (cast `/Game/Blueprints/player_BP` OtherActor)
  (`self.DisableInput` null)
  (`Widget.RemoveFromParent` (stale `self.Box.OnComponentBeginOverlap` _returnvalue)))

(fn `UserConstructionScript`)