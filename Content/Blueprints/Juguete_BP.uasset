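; Interactable toy actor that shows the JuanCarlos_IF widget and plays a sound when the player uses it.
; A box overlap with player_BP enables input and shows the Interacción_IF prompt, and leaving disables input and removes it.
; The Interacción action swaps the prompt for JuanCarlos_IF, plays OHMYGAH_ as a 2D sound after a delay, then removes the widget after a second delay.
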(event `InputAction|Interacción`
  (params (Key :type "Key Structure"))
  ;[1 1 1] Mensaje e interacción
  (:`Pressed`
    (`Widget.RemoveFromParent` (stale `self.Box.OnComponentBeginOverlap` _returnvalue))
    (bind _returnvalue (`|CreateWidget` "/Game/Interfaces/JuanCarlos_IF.JuanCarlos_IF_C"))
    (`UserWidget.AddToViewport` _returnvalue 0)
    (`KismetSystemLibrary.Delay` 2.5)
    (`GameplayStatics.PlaySound2D` "/Game/Sonidos/OH-MY-GAH_.OH-MY-GAH_" 0.75 1.0 0.0 null null)
    (`KismetSystemLibrary.Delay` 1.5)
    (`Widget.RemoveFromParent` _returnvalue)))

(event `self.Box.OnComponentBeginOverlap`
  (params (OverlappedComponent :type "PrimitiveComponent Object Reference") (OtherActor :type "Actor Object Reference") (OtherComp :type "PrimitiveComponent Object Reference") (OtherBodyIndex :type Integer) (bFromSweep :type Boolean) (SweepResult :type "HitResult Structure (by ref)"))
  ;[1 1 1] Mensaje e interacción
  (cast `/Game/Blueprints/player_BP` OtherActor)
  (`self.EnableInput` (`GameplayStatics.GetPlayerController` 0))
  (bind _returnvalue (`|CreateWidget` "/Game/Interfaces/Interacción_IF.Interacción_IF_C"))
  (`UserWidget.AddToViewport` _returnvalue 0))

(event `self.Box.OnComponentEndOverlap`
  (params (OverlappedComponent :type "PrimitiveComponent Object Reference") (OtherActor :type "Actor Object Reference") (OtherComp :type "PrimitiveComponent Object Reference") (OtherBodyIndex :type Integer))
  ;[1 1 1] Mensaje e interacción
  (cast `/Game/Blueprints/player_BP` OtherActor)
  (`self.DisableInput` null)
  (`Widget.RemoveFromParent` (stale `self.Box.OnComponentBeginOverlap` _returnvalue)))

(fn `UserConstructionScript`)